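; BP_Rock is a damageable rock actor that places itself on the terrain when play begins.
; BeginPlay caches the spawn and terrain actors, then lifts the rock high and lets ComponentPutInGround either reposition or destroy it.
; Life scales with the rock's X scale, and TakeDamage sets it to damage minus Life (operands look reversed), destroying the rock at zero or below.
; An older line-trace placement with water and tree checks remains unconnected.
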(event EventBeginPlay
  (bind _outactors (Actor|GetAllActorsOfClass "/Game/Actors/Tools/BP_SpawnObject.BP_SpawnObject_C"))
  (Variables|Default|SetSpawn (Utilities|Array|Get(acopy) _outactors))
  (bind _outactors_2 (Actor|GetAllActorsOfClass "/Game/Actors/Grid/BP_Terrain.BP_Terrain_C"))
  (Variables|Default|SetTerrain (Utilities|Array|Get(acopy) _outactors_2))
  (CallFunction|PutRockinGround)
  (Variables|Default|Setlife (* 3.0 (.x (Transformation|GetWorldScale (Variables|Default|GetDefaultSceneRoot))))))

(fn ConstructionScript)

(fn PutRockinGround
  (bind _rock (Variables|Default|GetRock))
  (bind _returnvalue (Transformation|GetWorldLocation _rock))
  (Transformation|Teleport (Math|Vector|MakeVector (.x _returnvalue) (.y _returnvalue) 6e+03) "0, 0, 0")
  (bind (_newposition _destroy) (Default|PutinGround (Variables|Default|GetComponent_PutInGround) self))
  (if _destroy
    (Actor|DestroyActor)
    (else
      (Transformation|Teleport _newposition "0, 0, 0"))))

(fn TakeDamage
  (params (takeDamage :type Float%20%28single-precision%29))
  (bind _output_get (Variables|Default|Setlife (- takeDamage (Variables|Default|Getlife))))
  (if (<= _output_get 0.0)
    (Actor|DestroyActor)))