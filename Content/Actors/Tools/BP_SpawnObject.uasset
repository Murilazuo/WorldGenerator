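; Spawner tool that scatters ToSpawn actors at random over the level's BP_Terrain.
; Shortly after BeginPlay it finds the terrain and spawns a count scaled by terrain area and Density, tracked in Objects.
; Each gets a random X/Y within the terrain bounds, a fixed high Z and independent per-axis scale from ScaleSize.
; ResetLevel destroys every actor of that class and respawns the set.
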(event EventBeginPlay
  (Utilities|FlowControl|Delay 0.3)
  (bind _outactors (Actor|GetAllActorsOfClass "/Game/Actors/Grid/BP_Terrain.BP_Terrain_C"))
  (Variables|Default|SetRef_Terrain (Utilities|Array|Get(acopy) _outactors))
  (CallFunction|SpawnAllObjects))

(fn ConstructionScript)

(fn SpawnObject
  (bind (_randomscale _randomposition) (CallFunction|GenerateSpawnTransform))
  (bind _returnvalue (Game|SpawnActorfromClass (Variables|Default|GetToSpawn) (Math|Transform|MakeTransform _randomposition "0, 0, 0" _randomscale) "Undefined" 0 0))
  (Utilities|Array|Add (Variables|Default|GetObjects) _returnvalue))

(fn GenerateSpawnTransform
  (bind _scalesize (Variables|Default|GetScaleSize))
  (bind _ref_terrain (Variables|Default|GetRef_Terrain))
  (bind _returnvalue (Math|Random|RandomFloatinRange (.x _scalesize) (.y _scalesize)))
  (bind _distancetovertex (Variables|/Game/Actors/Grid/BP_Terrain.BP_Terrain_C|GetDistanceToVertex _ref_terrain))
  (return (Math|Vector|MakeVector _returnvalue _returnvalue _returnvalue) (Math|Vector|MakeVector (Math|Random|RandomFloatinRange 0.0 (* (Variables|/Game/Actors/Grid/BP_Terrain.BP_Terrain_C|GetSizeX _ref_terrain) _distancetovertex)) (Math|Random|RandomFloatinRange 0.0 (* (Variables|/Game/Actors/Grid/BP_Terrain.BP_Terrain_C|GetSizeY _ref_terrain) _distancetovertex)) 6e+03)))

(fn ResetLevel
  (bind _outactors (Actor|GetAllActorsOfClass (Variables|Default|GetToSpawn)))
  (for _array_element _outactors
    (Actor|DestroyActor _array_element))
  (CallFunction|SpawnAllObjects))

(fn SpawnAllObjects
  (bind _ref_terrain (Variables|Default|GetRef_Terrain))
  (Utilities|Array|Clear (Variables|Default|GetObjects))
  (for _index (range 0 (* (/ (* (Variables|/Game/Actors/Grid/BP_Terrain.BP_Terrain_C|GetSizeX _ref_terrain) (Variables|/Game/Actors/Grid/BP_Terrain.BP_Terrain_C|GetSizeY _ref_terrain)) 100) (Variables|Default|GetDensity)))
    (CallFunction|SpawnObject)))