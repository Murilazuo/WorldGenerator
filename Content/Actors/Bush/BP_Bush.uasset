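; BP_Bush is a bush actor that places itself on the ground at BeginPlay and can take damage.
; It teleports to a height of 6000 at its X/Y, then ComponentPutInGround either supplies a new position, applied with zero rotation, or flags it for destruction.
; TakeDamage sets Life to Damage minus Life, an apparently reversed subtraction, and destroys the actor at zero or below.
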(event EventBeginPlay
  (bind _defaultsceneroot (Variables|Default|GetDefaultSceneRoot))
  (bind _returnvalue (Transformation|GetWorldLocation _defaultsceneroot))
  (Transformation|Teleport (Math|Vector|MakeVector (.x _returnvalue) (.y _returnvalue) 6e+03) "0, 0, 0")
  (bind (_newposition _destroy) (Default|PutinGround (Variables|Default|GetComponent_PutInGround) self))
  (if _destroy
    (Actor|DestroyActor)
    (else
      (Transformation|Teleport _newposition "0, 0, 0"))))

(event Collision|EventActorBeginOverlap
  (params (OtherActor :type Actor%20Object%20Reference)))

(event EventTick
  (params (DeltaSeconds :type Float%20%28single-precision%29)))

(fn ConstructionScript)

(fn TakeDamage
  (params (damage :type Float%20%28single-precision%29))
  (bind _output_get (Variables|Default|Setlife (- damage (Variables|Default|Getlife))))
  (if (<= _output_get 0.0)
    (Actor|DestroyActor)))