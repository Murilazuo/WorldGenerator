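; BP_Terrain is a procedural terrain actor that builds a random heightmap mesh with collision in its construction script.
; Random heights with fixed borders are smoothed by a clamped 3x3 neighbour average, then turned into grid vertices, triangles and tangents for a ProceduralMesh.
; ChangeTerrain raises or lowers the raw noise at CoordTerrain, then re-smooths and rebuilds the whole mesh.
; CreateWater only sets WaterHeight; its water-plane mesh code is disconnected.
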(fn ConstructionScript
  (CallFunction|CreateTerrain))

(fn GenerateNoise
  (bind _y (LocalVariables|GetY))
  (bind _y_2 (LocalVariables|GetY))
  (Utilities|Array|Clear (Variables|Default|GetRandomNoise))
  (for _index (range 0 (Variables|Default|GetSizeX))
    (for _index_2 (range 0 (Variables|Default|GetSizeY))
      (if (Math|Boolean|ORBoolean (== _index 0) (== _index_2 0) (== _index_2 (Variables|Default|GetSizeX)) (== _index (Variables|Default|GetSizeY)))
        (Utilities|Array|Add _y 1e+03)
        (else
          (Utilities|Array|Add _y (Math|Conversions|ToFloat(Integer) (Math|Float|Truncate (* (Variables|Default|GetHeight) (Math|Random|RandomFloat))))))))
    (Utilities|Array|Add (Variables|Default|GetRandomNoise) (Utilities|Struct|MakeNoiseMap _y_2))
    (Utilities|Array|Clear _y_2)))

(fn SmothNoise
  (bind _y (LocalVariables|GetY))
  (Utilities|Array|Clear (Variables|Default|GetNoiseMap))
  (for _index (range 0 (Variables|Default|GetSizeX))
    (LocalVariables|SetindexX _index)
    (for _index_2 (range 0 (Variables|Default|GetSizeY))
      (LocalVariables|SetindexY _index_2)
      (Utilities|FlowControl|Sequence
        (:then_0
          (bind _value (CallFunction|GetRandomNoisePosition (LocalVariables|GetindexX) (LocalVariables|GetindexY) 1)))
        (:then_1
          (bind _value_2 (CallFunction|GetRandomNoisePosition (LocalVariables|GetindexX) (LocalVariables|GetindexY) 1 1)))
        (:then_2
          (bind _value_3 (CallFunction|GetRandomNoisePosition (LocalVariables|GetindexX) (LocalVariables|GetindexY) 0 1)))
        (:then_3
          (bind _value_4 (CallFunction|GetRandomNoisePosition (LocalVariables|GetindexX) (LocalVariables|GetindexY) -1)))
        (:then_4
          (bind _value_5 (CallFunction|GetRandomNoisePosition (LocalVariables|GetindexX) (LocalVariables|GetindexY) -1 -1)))
        (:then_5
          (bind _value_6 (CallFunction|GetRandomNoisePosition (LocalVariables|GetindexX) (LocalVariables|GetindexY) 0 -1)))
        (:then_6
          (bind _value_7 (CallFunction|GetRandomNoisePosition (LocalVariables|GetindexX) (LocalVariables|GetindexY) 1 -1)))
        (:then_7
          (bind _value_8 (CallFunction|GetRandomNoisePosition (LocalVariables|GetindexX) (LocalVariables|GetindexY) -1 1)))
        (:then_8
          (bind _value_9 (CallFunction|GetRandomNoisePosition (LocalVariables|GetindexX) (LocalVariables|GetindexY)))
          (Utilities|Array|Add (LocalVariables|GetY) (Math|Float|Clamp(Float) (/ (+ _value _value_2 _value_4 _value_5 _value_6 _value_7 _value_8 _value_9 _value_3) 9.0) (Variables|Default|GetMinHeight) (Variables|Default|GetMaxHeight))))))
    (Utilities|Array|Add (Variables|Default|GetNoiseMap) (Utilities|Struct|MakeNoiseMap _y))
    (Utilities|Array|Clear _y)))

(fn GetRandomNoisePosition
  (params (X :type Integer) (Y :type Integer) (XtoAdd :type Integer) (YtoAdd :type Integer))
  (return (Utilities|Array|Get(acopy) (.y (Utilities|Array|Get(acopy) (Variables|Default|GetRandomNoise) (Math|Integer|Clamp(Integer) (+ X XtoAdd) 0 (Variables|Default|GetSizeX)))) (Math|Integer|Clamp(Integer) (+ Y YtoAdd) 0 (Variables|Default|GetSizeY)))))

(fn CreateMeshData
  (bind _distancetovertex (Variables|Default|GetDistanceToVertex))
  (Utilities|FlowControl|Sequence
    (:then_0
      (Utilities|Array|Clear (Variables|Default|GetVertex)))
    (:then_1
      (Utilities|Array|Clear (Variables|Default|GetTriangle)))
    (:then_2
      (Utilities|Array|Clear (Variables|Default|GetNormals)))
    (:then_3
      (Utilities|Array|Clear (Variables|Default|GetUV))
      (Utilities|Array|Clear (Variables|Default|GetTangents))
      (for _index (range 0 (Variables|Default|GetSizeX))
        (LocalVariables|SetX _index)
        (for _index_2 (range 0 (Variables|Default|GetSizeY))
          (LocalVariables|SetY _index_2)
          (Utilities|FlowControl|Sequence
            (:then_0
              (bind _value (CallFunction|GetNoisePosition (LocalVariables|GetX) (LocalVariables|GetY)))
              (Utilities|Array|Add (Variables|Default|GetVertex) (Math|Vector|MakeVector (* (LocalVariables|GetX) _distancetovertex) (* (LocalVariables|GetY) _distancetovertex) _value)))
            (:then_1
              (Utilities|Array|Add (Variables|Default|GetUV) (Math|Vector2D|MakeVector2D (Math|Conversions|ToFloat(Integer) (LocalVariables|GetX)) (Math|Conversions|ToFloat(Integer) (LocalVariables|GetY))))))))
      (Utilities|FlowControl|Sequence
        (:then_0
          (bind _triangles (Class|KismetProceduralMeshLibrary|CreateGridMeshTriangles (+ (Variables|Default|GetSizeX) 1) (+ (Variables|Default|GetSizeY) 1) false))
          (Variables|Default|SetTriangle _triangles))
        (:then_1
          (bind (_normals _tangents) (Class|KismetProceduralMeshLibrary|CalculateTangentsforMesh (Variables|Default|GetVertex) (Variables|Default|GetTriangle) (Variables|Default|GetUV)))
          (Variables|Default|SetNormals _normals)
          (Variables|Default|SetTangents _tangents))))))

(fn CreateTerrain
  (Utilities|FlowControl|Sequence
    (:then_0
      (CallFunction|GenerateNoise)
      (CallFunction|SmothNoise)
      (CallFunction|CreateMeshData))
    (:then_1
      (Rendering|Material|SetMaterial (Variables|Default|GetProceduralMesh) 0 "/Game/Actors/Terrain/M_Terrain.M_Terrain")
      (CallFunction|UpdateMesh)
      (CallFunction|CreateWater))))

(fn GetNoisePosition
  (params (X :type Integer) (Y :type Integer))
  (return (Utilities|Array|Get(acopy) (.y (Utilities|Array|Get(acopy) (Variables|Default|GetNoiseMap) X)) Y)))

(fn CreateWater
  (Variables|Default|SetWaterHeight 2.1e+03))

(fn UpdateMesh
  (Class|ProceduralMeshComponent|CreateMeshSectionLinearColor (Variables|Default|GetProceduralMesh) 0 (Variables|Default|GetVertex) (Variables|Default|GetTriangle) (Variables|Default|GetNormals) (Variables|Default|GetUV) 0 0 0 0 (Variables|Default|GetTangents) true))

(fn ChangeTerrain
  (params (toAddZ :type Float%20%28single-precision%29) (CoordTerrain :type Vector) (Increment :type Boolean))
  (bind _distancetovertex (Variables|Default|GetDistanceToVertex))
  (CallFunction|AddRandomNoisePosition (Math|Float|Truncate (/ (.x CoordTerrain) _distancetovertex)) (Math|Float|Truncate (/ (.y CoordTerrain) _distancetovertex)) toAddZ Increment)
  (CallFunction|SmothNoise)
  (CallFunction|CreateMeshData)
  (CallFunction|UpdateMesh))

(fn AddRandomNoisePosition
  (params (X :type Integer) (Y :type Integer) (ToAdd :type Float%20%28single-precision%29) (Increment :type Boolean))
  (bind _returnvalue (Math|Float|Truncate ToAdd))
  (bind _randomnoise (Variables|Default|GetRandomNoise))
  (bind _output (Utilities|Array|Get(acopy) _randomnoise X))
  (bind _output_2 (Utilities|Array|Get(acopy) (.y _output) Y))
  (if Increment
    (for _index (range 0 _returnvalue)
      (Math|Float|IncrementFloat _output_2))
    (else
      (for _index_2 (range 0 _returnvalue)
        (Math|Float|DecrementFloat _output_2)))))